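; Interactable actor that, when a TopDownCharacter overlaps its box, is either collected into the inventory and destroyed or checks required items.
; Required item quantities are compared with the character's inventory map, marking RequirementsMet and firing the interaction event once none are false.
; A DoOnce and gate size that array on first overlap, then route later overlaps straight to the check.
; Non-collectables without requirements do nothing; CheckRequirements is an empty stub.
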(event OnComponentBeginOverlap(Box)
  (params (OverlappedComponent :type Primitive%20Component%20Object%20Reference) (OtherActor :type Actor%20Object%20Reference) (OtherComp :type Primitive%20Component%20Object%20Reference) (OtherBodyIndex :type Integer) (bFromSweep :type Boolean) (SweepResult :type Hit%20Result%20Structure%20%28by%20ref%29))
  (bind _requireditemstoquantities (Variables|InteractableData|GetrequiredItemsToQuantities))
  (bind _returnvalue (Utilities|Map|Length _requireditemstoquantities))
  (bind _astop_down_character (Utilities|Casting|CastToTopDownCharacter OtherActor))
  (if (Variables|InteractableData|GetisCollectable) ; If true, object will be collected and destroyed.
    (Default|UpdateInventory _astop_down_character "BP_Interactable_C")
    (Actor|DestroyActor)
    (else
      ;[1 1 1] Check if there are any required items
      (if (> _returnvalue 0)
        ;[1 1 1] Execute array expansion once
        (Utilities|FlowControl|Sequence
          (:then_0
            (Utilities|FlowControl|Gate true :!label _label
              (:Exit
                _)))
          (:then_1
            (Utilities|FlowControl|DoOnce false
              (:Completed
                (Utilities|FlowControl|Sequence
                  (:then_0
                    ;[1 1 1] Expand confirmation array to no. required items
                    (for _index (range _returnvalue 1)
                      (Utilities|Array|Add (Variables|InteractableData|GetrequirementsMet) false)))
                  (:then_1
                    (goto _label Open)))))))
        ;[1 1 1] Find if the required item exists in the inventory
        (bind _keys (Utilities|Map|Keys _requireditemstoquantities))
        (for (_array_element _array_index) _keys
          (if (.ReturnValue (Utilities|Map|Find (Variables|/Game/TopDownBP/Blueprints/TopDownCharacter.TopDownCharacter_C|GetinventoryActorsToInt _astop_down_character) _array_element))
            ;[1 1 1] Find if the number of items in the inventory meet the requirements
            (bind _values (Utilities|Map|Values _requireditemstoquantities))
            (if (>= (.Value (Utilities|Map|Find (Variables|/Game/TopDownBP/Blueprints/TopDownCharacter.TopDownCharacter_C|GetinventoryActorsToInt _astop_down_character) _array_element)) (Utilities|Array|Get(acopy) _values _array_index))
              ;[1 1 1] Update inventory requirements
              (Utilities|Array|SetArrayElem (Variables|InteractableData|GetrequirementsMet) _array_index true))))
        ;[1 1 1] Check if all requirements are met
        (if (not (Utilities|Array|ContainsItem (Variables|InteractableData|GetrequirementsMet) false))
          ;[1 1 1] Call interaction event
          (Default|CallInteractionEvent))))))

(fn ConstructionScript)

(fn CheckRequirements
  (params (player :type Top%20Down%20Character%20Object%20Reference)))