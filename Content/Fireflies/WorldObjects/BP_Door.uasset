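; BP_Door is a world door that swings open and closed through Door_Open and Door_Close events.
; The construction script caches the Scene component's world rotation as the initial rotation.
; A DoorRotate timeline drives a shortest-path lerp from that rotation to one combined with DoorRotation.
; Opening plays the timeline from the start and closing reverses it from the end, so either call restarts from an endpoint.
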(event Custom|Door_Open
  (bind _initrotation (Variables|Default|GetinitRotation))
  (bind _alpha (Timeline|DoorRotate PlayFromStart)
    (:Update
      (Transformation|SetWorldRotation (Variables|Default|GetScene) (Math|Rotator|Lerp(Rotator) _initrotation (Math|Rotator|CombineRotators _initrotation (Variables|Default|GetdoorRotation)) _alpha true) false false))))

(event Custom|Door_Close
  (bind _initrotation (Variables|Default|GetinitRotation))
  (bind _alpha (Timeline|DoorRotate ReverseFromEnd)
    (:Update
      (Transformation|SetWorldRotation (Variables|Default|GetScene) (Math|Rotator|Lerp(Rotator) _initrotation (Math|Rotator|CombineRotators _initrotation (Variables|Default|GetdoorRotation)) _alpha true) false false))))

(fn ConstructionScript
  ;[1 1 1] Update the initial rotation based on world transform
  (Variables|Default|SetinitRotation (Transformation|GetWorldRotation (Variables|Default|GetScene))))