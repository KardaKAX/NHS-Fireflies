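; BP_Fireflies is a world firefly that loops along a spline and reacts when the top-down character reaches it.
; A timeline drives the mesh along the spline, with play rate set from LoopTime, restarting when finished.
; Overlapping Box1 briefly sets the character's Swinging flag and plays once-gated whoosh and jar-close sounds, while AudioTrigger plays a firefly sound.
; A bound destroy event hides mesh and trail, disables collision, then destroys the actor after a delay.
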(event OnComponentBeginOverlap(Box1)
  (params (OverlappedComponent :type Primitive%20Component%20Object%20Reference) (OtherActor :type Actor%20Object%20Reference) (OtherComp :type Primitive%20Component%20Object%20Reference) (OtherBodyIndex :type Integer) (bFromSweep :type Boolean) (SweepResult :type Hit%20Result%20Structure%20%28by%20ref%29))
  (bind _returnvalue (Transformation|GetActorLocation))
  (bind _astop_down_character (Utilities|Casting|CastToTopDownCharacter OtherActor))
  (Utilities|FlowControl|Sequence
    (:then_0
      (Variables|/Game/TopDownBP/Blueprints/TopDownCharacter.TopDownCharacter_C|SetSwinging? _astop_down_character true)
      (Utilities|FlowControl|Delay 1.0)
      (Variables|/Game/TopDownBP/Blueprints/TopDownCharacter.TopDownCharacter_C|SetSwinging? _astop_down_character false)
      (Utilities|FlowControl|DoOnce false
        (:Completed
          (Audio|PlaySoundatLocation "/Game/Assets/Sounds/JarClose.JarClose" _returnvalue "0, 0, 0" 1.0 1.0 0.0 0 0 0))))
    (:then_1
      (Utilities|FlowControl|DoOnce false
        (:Completed
          (Utilities|FlowControl|Delay 0.2)
          (Audio|PlaySoundatLocation "/Game/Assets/Sounds/Whoosh1.Whoosh1" _returnvalue "0, 0, 0" 1.0 1.0 0.0 0 0 0))))))

(event OnComponentBeginOverlap(AudioTrigger)
  (params (OverlappedComponent :type Primitive%20Component%20Object%20Reference) (OtherActor :type Actor%20Object%20Reference) (OtherComp :type Primitive%20Component%20Object%20Reference) (OtherBodyIndex :type Integer) (bFromSweep :type Boolean) (SweepResult :type Hit%20Result%20Structure%20%28by%20ref%29))
  (Utilities|FlowControl|DoOnce false
    (:Completed
      (Audio|PlaySoundatLocation "/Game/Assets/Sounds/Firefly.Firefly" (Transformation|GetWorldLocation (Variables|Default|GetStaticMesh)) "0, 0, 0" 0.8 1.0 0.0 0 0 0))))

(event Custom|FireFlyDestroy
  (bind _returnvalue (Transformation|GetActorLocation))
  (Rendering|SetVisibility (Variables|Default|GetStaticMesh) false false)
  (Collision|SetCollisionEnabled (Variables|Default|GetBox) "NoCollision")
  (Utilities|FlowControl|Delay 2.0)
  (Actor|DestroyActor)
  (Utilities|FlowControl|Sequence
    (:then_0
      (Utilities|FlowControl|DoOnce false) ; enters at Reset
    )
    (:then_1
      (Utilities|FlowControl|DoOnce false) ; enters at Reset
    )))

(event EventBeginPlay
  (bind _spline (Variables|Default|GetSpline))
  (Utilities|FlowControl|Sequence
    (:then_0
      (Variables|Default|SetDelay 2.0)
      (Components|Timeline|SetPlayRate (Variables|Default|GetTL_FireflyMovement) (/ 1.0 (Variables|Default|GetloopTime)))
      (bind _alpha (Timeline|TL_FireflyMovement PlayFromStart)
        (:Update
          (Transformation|SetWorldTransform (Variables|Default|GetStaticMesh) (Math|Transform|MakeTransform (.location (Spline|GetTransformatDistanceAlongSpline _spline (* _alpha (Spline|GetSplineLength _spline)) "World" false)) (Math|Rotator|CombineRotators (.rotation (Spline|GetTransformatDistanceAlongSpline _spline (* _alpha (Spline|GetSplineLength _spline)) "World" false)) "0,90.000000, 0") (.scale (Spline|GetTransformatDistanceAlongSpline _spline (* _alpha (Spline|GetSplineLength _spline)) "World" false))) false false))
        (:Finished
          (Timeline|TL_FireflyMovement PlayFromStart))))
    (:then_1
      (EventDispatchers|BindEventtoDestroyEvent (delegate Custom|FireFlyDestroy)))))

(fn ConstructionScript
  (|CallParentFunction))