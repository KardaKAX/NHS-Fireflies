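; BP_Flamebug is a world object whose static mesh flies endlessly along a spline path.
; A restarting timeline drives distance along the spline, with LoopTime setting the play rate and a fixed 90-degree offset applied to the mesh rotation.
; When a TopDownCharacter begins overlapping Box1, its Swinging flag is set true, then cleared after a one-second delay.
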(event OnComponentBeginOverlap(Box1)
  (params (OverlappedComponent :type Primitive%20Component%20Object%20Reference) (OtherActor :type Actor%20Object%20Reference) (OtherComp :type Primitive%20Component%20Object%20Reference) (OtherBodyIndex :type Integer) (bFromSweep :type Boolean) (SweepResult :type Hit%20Result%20Structure%20%28by%20ref%29))
  (bind _astop_down_character (Utilities|Casting|CastToTopDownCharacter OtherActor))
  (Variables|/Game/TopDownBP/Blueprints/TopDownCharacter.TopDownCharacter_C|SetSwinging? _astop_down_character true)
  (Utilities|FlowControl|Delay 1.0)
  (Variables|/Game/TopDownBP/Blueprints/TopDownCharacter.TopDownCharacter_C|SetSwinging? _astop_down_character false))

(event EventBeginPlay
  (bind _spline (Variables|Default|GetSpline))
  (Variables|Default|SetDelay 2.0)
  (Components|Timeline|SetPlayRate (Variables|Default|GetTL_FireflyMovement) (/ 1.0 (Variables|Default|GetloopTime)))
  (bind _alpha (Timeline|TL_FireflyMovement PlayFromStart)
    (:Update
      (Transformation|SetWorldTransform (Variables|Default|GetStaticMesh) (Math|Transform|MakeTransform (.location (Spline|GetTransformatDistanceAlongSpline _spline (* _alpha (Spline|GetSplineLength _spline)) "World" false)) (Math|Rotator|CombineRotators (.rotation (Spline|GetTransformatDistanceAlongSpline _spline (* _alpha (Spline|GetSplineLength _spline)) "World" false)) "0,90.000000,0.000000") (.scale (Spline|GetTransformatDistanceAlongSpline _spline (* _alpha (Spline|GetSplineLength _spline)) "World" false))) false false))
    (:Finished
      (Timeline|TL_FireflyMovement PlayFromStart))))

(fn ConstructionScript
  (|CallParentFunction))