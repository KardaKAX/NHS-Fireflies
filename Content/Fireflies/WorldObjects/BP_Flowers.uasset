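; BP_Flowers is a world object that scatters randomized flower meshes within a configurable box area.
; Its construction script sizes the box, then creates instanced static mesh components, each given a random mesh and random materials per slot.
; It then distributes the requested instance count randomly across those components, keeping variety within a few instanced components.
; A helper builds each transform from a random XY point in the box bounds, with random yaw and per-axis scale.
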(fn ConstructionScript
  ;[1 1 1] Set area to render within
  (Components|Box|SetBoxExtent (Variables|Default|GetBox) (Variables|Construction|GetmeshArea) true)
  ;[1 1 1] For each variation desired...
  (for _index (range 1 (Variables|Construction|GetmeshVariation))
    ;[1 1 1] Add a random mesh type
    (bind _returnvalue (AddComponent|AddInstancedStaticMeshComponent false))
    (Components|StaticMesh|SetStaticMesh _returnvalue (Utilities|RandominArray (Variables|Construction|GetmeshTypes)))
    ;[1 1 1] Add ISM to array
    (Utilities|Array|Add (LocalVariables|GetinstancedMeshes) _returnvalue)
    ;[1 1 1] Set material elements on mesh
    (for _index_2 (range 1 (Rendering|Material|GetNumMaterials _returnvalue))
      (Rendering|Material|SetMaterial _returnvalue (- _index_2 1) (Utilities|RandominArray (Variables|Construction|GetmaterialTypes)))))
  ;[1 1 1] For the number of desired meshes...
  (for _index_3 (range 1 (Variables|Construction|GetmeshCount))
    ;[1 1 1] Add an instance to a random available type
    (Components|InstancedStaticMesh|AddInstance (Utilities|RandominArray (LocalVariables|GetinstancedMeshes)) (Utilities|RandomTransforminRange (Variables|Default|GetBox)))))