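; Interactable toad that hurts players who lack fireflies and can be killed through its interaction event.
; The bound interaction event plays the death animation and sound, then destroys the actor after a short delay.
; Entering Sphere without fireflies in inventory plays a gendered grunt and briefly sets the character's TakingDamage flag for the damage animation.
; A separate Sound trigger plays a ribbit, throttled by a DoOnce that resets after a delay on exit.
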(event OnComponentBeginOverlap(Sphere)
  (params (OverlappedComponent :type Primitive%20Component%20Object%20Reference) (OtherActor :type Actor%20Object%20Reference) (OtherComp :type Primitive%20Component%20Object%20Reference) (OtherBodyIndex :type Integer) (bFromSweep :type Boolean) (SweepResult :type Hit%20Result%20Structure%20%28by%20ref%29))
  ;[1 1 1] Checks if player has flamebug
  (bind _astop_down_character (Utilities|Casting|CastToTopDownCharacter OtherActor))
  (if (not (>= (.Value (Utilities|Map|Find (Variables|/Game/TopDownBP/Blueprints/TopDownCharacter.TopDownCharacter_C|GetinventoryActorsToInt _astop_down_character) "/Game/Fireflies/WorldObjects/BP_Fireflies.BP_Fireflies_C")) 1))
    ;[1 1 1] Play damage animation if player does not
    (if (Variables|/Game/TopDownBP/Blueprints/TopDownCharacter.TopDownCharacter_C|GetBoy? _astop_down_character)
      (Audio|PlaySoundatLocation "/Game/Assets/Sounds/GruntMale.GruntMale" (Transformation|GetWorldLocation (Variables|/Script/Engine.Character|GetMesh _astop_down_character)) "0, 0, 0" 1.0 1.0 0.0 0 0 0)
      (else
        (Audio|PlaySoundatLocation "/Game/Assets/Sounds/GruntFemale.GruntFemale" (Transformation|GetWorldLocation (Variables|/Script/Engine.Character|GetMesh _astop_down_character)) "0, 0, 0" 1.0 1.0 0.0 0 0 0)))
    (Variables|/Game/TopDownBP/Blueprints/TopDownCharacter.TopDownCharacter_C|SetTakingDamage? _astop_down_character true)
    (Utilities|FlowControl|Delay 2.0)
    (Variables|/Game/TopDownBP/Blueprints/TopDownCharacter.TopDownCharacter_C|SetTakingDamage? _astop_down_character false)))

(event OnComponentEndOverlap(Sphere)
  (params (OverlappedComponent :type Primitive%20Component%20Object%20Reference) (OtherActor :type Actor%20Object%20Reference) (OtherComp :type Primitive%20Component%20Object%20Reference) (OtherBodyIndex :type Integer))
  ;[1 1 1] Stop damage animation
  (bind _astop_down_character (Utilities|Casting|CastToTopDownCharacter OtherActor))
  (Variables|/Game/TopDownBP/Blueprints/TopDownCharacter.TopDownCharacter_C|SetTakingDamage? _astop_down_character false))

(event OnComponentEndOverlap(Sound)
  (params (OverlappedComponent :type Primitive%20Component%20Object%20Reference) (OtherActor :type Actor%20Object%20Reference) (OtherComp :type Primitive%20Component%20Object%20Reference) (OtherBodyIndex :type Integer))
  ;[1 1 1] Plays ribbet
  (Utilities|FlowControl|Delay 6.0)
  (Utilities|FlowControl|DoOnce false) ; enters at Reset
)

(event OnComponentBeginOverlap(Sound)
  (params (OverlappedComponent :type Primitive%20Component%20Object%20Reference) (OtherActor :type Actor%20Object%20Reference) (OtherComp :type Primitive%20Component%20Object%20Reference) (OtherBodyIndex :type Integer) (bFromSweep :type Boolean) (SweepResult :type Hit%20Result%20Structure%20%28by%20ref%29))
  ;[1 1 1] Plays ribbet
  (Utilities|FlowControl|DoOnce false
    (:Completed
      (Audio|PlaySoundatLocation "/Game/Assets/Sounds/FrogRibbit.FrogRibbit" (Transformation|GetWorldLocation (Variables|Default|GetSkeletalMesh)) "0, 0, 0" 1.0 1.0 0.0 0 0 0))))

(event Custom|FrogDead
  ;[1 1 1] Death animation and sound
  (Components|Animation|PlayAnimation (Variables|Default|GetSkeletalMesh) "/Game/Assets/FrogAnimation/FrogDeath.FrogDeath" false)
  (Audio|PlaySoundatLocation "/Game/Assets/Sounds/FrogDying.FrogDying" (Transformation|GetWorldLocation (Variables|Default|GetSkeletalMesh)) "0, 0, 0" 1.0 1.0 0.0 0 0 0)
  ;[1 1 1] Destroy
  (Utilities|FlowControl|Delay 1.0)
  (Actor|DestroyActor))

(event EventBeginPlay
  (EventDispatchers|BindEventtoInteractionEvent (delegate Custom|FrogDead)))

(fn ConstructionScript
  (|CallParentFunction))