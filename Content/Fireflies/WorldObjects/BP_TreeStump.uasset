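; BP_TreeStump is an interactable world object that opens and closes the doors connected to it.
; On BeginPlay it binds its handler to an interaction event, which appears to come from a master parent Blueprint.
; Each interaction calls DoorOpen or DoorClose on every entry in ConnectedDoors according to TriggerState, then flips that flag for the next use.
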(event Custom|stumpInteraction_Event
  ;[1 1 1] Bind interaction event from master
  ;[1 1 1] Toggle connected door state
  (for _array_element (Variables|InteractableData|GetconnectedDoors)
    (if (Variables|InteractableData|GettriggerState)
      (Default|DoorOpen _array_element)
      (else
        (Default|DoorClose _array_element))))
  (Variables|InteractableData|SettriggerState (not (Variables|InteractableData|GettriggerState))))

(event EventBeginPlay
  ;[1 1 1] Bind interaction event from master
  (EventDispatchers|BindEventtoInteractionEvent (delegate Custom|stumpInteraction_Event)))

(fn ConstructionScript
  (|CallParentFunction))